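; BP_CashMachine is a cash machine that turns gold during buying time and drops an item when the first-person character overlaps it.
; It follows BP_GameManager state changes, counting each buying phase in WaveNumber.
; A count of one yields the first Items entry, otherwise a random one; that first pick or a random key resets the count.
; Each drop notifies BP_MachineManager, whose disable-all event it binds to.
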(event `self.ReceiveBeginPlay`
  (bind _returnvalue (`GameplayStatics.GetActorOfClass` "/Game/Game/MainLevel/BP_GameManager.BP_GameManager_C"))
  (add `/Game/Game/MainLevel/BP_GameManager.OnGameStateChanged` _returnvalue (delegate `EnableMachine`))
  (bind _returnvalue_2 (`GameplayStatics.GetActorOfClass` "/Game/Game/CashMachines/BP_MachineManager.BP_MachineManager_C"))
  (set `self.MachineManager` _returnvalue_2)
  (add `/Game/Game/CashMachines/BP_MachineManager.OnDisableAllMachines` _returnvalue_2 (`|CreateDelegate` :!event `DisableMachine`)))

(event `EnableMachine`
  (params (IsBuyingTime :type Boolean))
  (bind _sm_asset_cachemachine (`self.SM_Asset_CacheMachine`))
  (bind _output_get (set `self.IsActivated` IsBuyingTime))
  (if _output_get
    (`/Engine/EditorBlueprintResources/StandardMacros.IncrementInt` (`self.WaveNumber`)
      (:`  `
        (`PrimitiveComponent.SetMaterial` _sm_asset_cachemachine 0 "/Game/StarterContent/Materials/M_Metal_Gold.M_Metal_Gold")))
    (else
      (`PrimitiveComponent.SetMaterial` _sm_asset_cachemachine 0 "/Engine/MapTemplates/Materials/BasicAsset01.BasicAsset01" :!label _label))))

(event `DisableMachine`
  (set `self.IsActivated` false)
  (goto _label))

(event `self.Box.OnComponentBeginOverlap`
  (params (OverlappedComponent :type "PrimitiveComponent Object Reference") (OtherActor :type "Actor Object Reference") (OtherComp :type "PrimitiveComponent Object Reference") (OtherBodyIndex :type Integer) (bFromSweep :type Boolean) (SweepResult :type "HitResult Structure (by ref)"))
  (if (`self.IsActivated`)
    (cast `/Game/FirstPerson/Blueprints/BP_FirstPersonCharacter` OtherActor)
    (`self.Drop Item`)))

(event `Drop Item`
  (bind (_returnvalue_location _returnvalue_rotation _returnvalue_scale) (`KismetMathLibrary.BreakTransform` (`self.GetTransform`)))
  (`GameplayStatics.PlaySound2D` "/Game/Game/Assets/Sounds/cashMachine.cashMachine" 1.0 1.0 0.0 null null)
  (if (== (`self.WaveNumber`) 1)
    (set `self.WaveNumber` 0)
    (set `self.SpawnActor` (`|GetArrayItem` (`self.Items`)))
    (else
      (bind _output_get (set `self.SpawnActor` (`KismetArrayLibrary.Array_Random` (`self.Items`))))
      (castclass `/Game/Game/PowerUps/BP_Key` _output_get
        (:`then`
          (set `self.WaveNumber` 0))
        (:`CastFailed`
          _))))
  (`|SpawnActorFromClass` (`self.SpawnActor`) (`KismetMathLibrary.MakeTransform` (+ (+ _returnvalue_location (* (`KismetMathLibrary.GetForwardVector` _returnvalue_rotation) 150.0)) (0.0 0.0 50.0)) _returnvalue_rotation _returnvalue_scale) "Undefined" "MultiplyWithRoot" null null)
  (`/Game/Game/CashMachines/BP_MachineManager.OnMachineUsed` (`self.MachineManager`)))

(fn `UserConstructionScript`)