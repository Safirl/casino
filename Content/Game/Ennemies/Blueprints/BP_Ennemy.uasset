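; Card guard enemy that patrols, chases the sensed player and attacks, randomly tagged as Red or Black and registered with the player's matching render list.
; BeginPlay builds patrol points from the game manager's unlocked zone for the first destination; later ones come only from zone 0.
; PawnSensing switches Tick-driven patrol to an AIMoveTo chase.
; On arrival, a delayed line trace removes player HP and destroys the guard on a hit.
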(event `self.ReceiveBeginPlay`
  (bind _pawnsensing (`self.PawnSensing`))
  (bind _outitem (`KismetArrayLibrary.Array_Random` (`self.Choose_Team`)))
  (`|ExecutionSequence`
    (:`then_0`
      (if (not (`ActorComponent.IsActive` _pawnsensing))
        (`ActorComponent.SetActive` _pawnsensing true false)
        (bind _returnvalue (`GameplayStatics.GetActorOfClass` "/Game/Game/MainLevel/BP_GameManager.BP_GameManager_C"))
        (for _index (range (`/Game/Game/MainLevel/BP_GameManager.UnlockedZone` _returnvalue) 1)
          (switch `int` _index
            (:`0`
              (for _array_element (`self.TargetLocations_0`)
                (`KismetArrayLibrary.Array_Add` (`self.AllTargetLocations`) _array_element)))
            (:`1`
              (for _array_element_2 (`self.TargetLocations_1`)
                (`KismetArrayLibrary.Array_Add` (`self.AllTargetLocations`) _array_element_2)))
            (:`2`
              (for _array_element_3 (`self.TargetLocations_2`)
                (`KismetArrayLibrary.Array_Add` (`self.AllTargetLocations`) _array_element_3)))))
        (set `self.CurrentDestinationZone0` (`KismetArrayLibrary.Array_Random` (`self.AllTargetLocations`)))))
    (:`then_1`
      (set `self.Tags` (`|MakeArray` _outitem))
      (bind _returnvalue_2 (`GameplayStatics.GetActorOfClass` "/Game/FirstPerson/Blueprints/BP_FirstPersonCharacter.BP_FirstPersonCharacter_C"))
      (switch `name` _outitem
        (:`red`
          (`/Game/FirstPerson/Blueprints/BP_FirstPersonCharacter.AddRedToRender` _returnvalue_2 self))
        (:`black`
          (`/Game/FirstPerson/Blueprints/BP_FirstPersonCharacter.AddBlackToRender` _returnvalue_2 self))))))

(event `self.ReceiveTick`
  (params (DeltaSeconds :type "Float (single-precision)"))
  (if (not (or (`self.IsSeeingPlayer`) (`self.IsAttacking`)))
    (`|AIMoveTo` self (`self.CurrentDestinationZone0`) null 100.0
      (:`OnSuccess`
        (set `self.CurrentDestinationZone0` (`KismetArrayLibrary.Array_Random` (`self.TargetLocations_0`)))))))

(event `self.PawnSensing.OnSeePawn`
  (params (Pawn :type "Pawn Object Reference"))
  (`/Engine/EditorBlueprintResources/StandardMacros.IsValid` Pawn
    (:`Is Valid`
      (bind _asbp_first_person_character (cast `/Game/FirstPerson/Blueprints/BP_FirstPersonCharacter` Pawn))
      (set `self.TargetPawn` _asbp_first_person_character)
      (set `self.IsSeeingPlayer` true)
      (`self.FollowPlayer`))))

(event `FollowPlayer`
  (`MovementComponent.StopMovementImmediately` (`self.CharacterMovement`))
  (if (`self.IsAttacking`)
    (goto _label :!via `Reset`)
    (else
      (`|ExecutionSequence`
        (:`then_0`
          (`|AIMoveTo` self (0.0 0.0 0.0) (`self.TargetPawn`) 120.0
            (:`OnSuccess`
              (`self.Server_Attack`))))
        (:`then_1`
          (`/Engine/EditorBlueprintResources/StandardMacros.DoOnce` false :!label _label
            (:`Completed`
              (`SkeletalMeshComponent.PlayAnimation` (`self.SkeletalMesh`) "/Game/Game/Ennemies/Skeletal/CardGuard_walk.CardGuard_walk" true))))))))

(event `Server_Attack`
  (bind _scene (`self.Scene`))
  (bind _returnvalue (`SceneComponent.K2_GetComponentLocation` _scene))
  (`MovementComponent.StopMovementImmediately` (`self.CharacterMovement`))
  (set `self.IsAttacking` true)
  (set `self.IsSeeingPlayer` false)
  (`SkeletalMeshComponent.PlayAnimation` (`self.SkeletalMesh`) "/Game/Game/Ennemies/Skeletal/CardGuard_Atk.CardGuard_Atk" false)
  (`KismetSystemLibrary.Delay` 0.7)
  (bind _outhit (`KismetSystemLibrary.LineTraceSingle` :`Start` _returnvalue :`End` (+ (+ _returnvalue (0.0 0.0 -50.0)) (* 10000.0 (`SceneComponent.GetUpVector` _scene))) :`TraceChannel` "TraceTypeQuery1" :`DrawDebugType` "ForDuration"))
  (if (== (`GameplayStatics.GetObjectClass` (`.HitActor` (`GameplayStatics.BreakHitResult` _outhit))) "/Game/FirstPerson/Blueprints/BP_FirstPersonCharacter.BP_FirstPersonCharacter_C")
    (`KismetSystemLibrary.PrintString` "Touched")
    (bind _returnvalue_2 (`GameplayStatics.GetActorOfClass` "/Game/FirstPerson/Blueprints/BP_FirstPersonCharacter.BP_FirstPersonCharacter_C"))
    (set `/Game/FirstPerson/Blueprints/BP_FirstPersonCharacter.HP` (- (`/Game/FirstPerson/Blueprints/BP_FirstPersonCharacter.HP` _returnvalue_2) 1.0) _returnvalue_2)
    (`self.K2_DestroyActor`)
    (`KismetSystemLibrary.Delay` 0.4)
    (set `self.IsAttacking` false)))

(fn `UserConstructionScript`)