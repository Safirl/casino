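; BP_I_see_u is a scene-capture actor in the enemy PPV folder that renders a filtered view of the level.
; Its construction script creates a full-HD render target for the SceneCaptureComponent2D and adds actors tagged "Bati" to the capture's show-only components.
; InvertColor selects whether actors tagged "red" or "black" are also added.
; All setup happens at construction, with no active event logic.
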(event `self.ReceiveTick`
  (params (DeltaSeconds :type "Float (single-precision)")))

(fn `UserConstructionScript`
  (bind _returnvalue (`KismetRenderingLibrary.CreateRenderTarget2D` 1920 1080))
  (set `SceneCaptureComponent2D.TextureTarget` _returnvalue (`self.SceneCaptureComponent2D`))
  (bind _outactors (`GameplayStatics.GetAllActorsWithTag` "Bati"))
  (for _array_element _outactors
    (`SceneCaptureComponent.ShowOnlyActorComponents` (`self.SceneCaptureComponent2D`) _array_element false))
  (if (`self.Invert Color`)
    (bind _outactors_2 (`GameplayStatics.GetAllActorsWithTag` "red"))
    (for _array_element_2 _outactors_2
      (`SceneCaptureComponent.ShowOnlyActorComponents` (`self.SceneCaptureComponent2D`) _array_element_2 false))
    (else
      (bind _outactors_3 (`GameplayStatics.GetAllActorsWithTag` "black"))
      (for _array_element_3 _outactors_3
        (`SceneCaptureComponent.ShowOnlyActorComponents` (`self.SceneCaptureComponent2D`) _array_element_3 false)))))