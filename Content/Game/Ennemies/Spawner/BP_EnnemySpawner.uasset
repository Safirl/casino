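; Enemy spawner actor that registers with BP_SpawnerManager, waiting for BP_GameManager's creation event if none exists yet, and binds to its wave-start event.
; PopulateSpawner sets the enemy count, and SpawnEnnemies starts spawning after a zone check.
; SpawnSequence recursively spawns BP_Ennemy with a default controller, pausing randomly between spawns and offsetting height by the loop index times the spawner's Z.
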(event `OnSpawnerManagerCreated`
  (params (SpawnerManager :type "/Game/Game/Ennemies/Spawner/BP_SpawnerManager Object Reference"))
  (`/Game/Game/Ennemies/Spawner/BP_SpawnerManager.OnSpawnerAdded` SpawnerManager self)
  (add `/Game/Game/Ennemies/Spawner/BP_SpawnerManager.OnWaveStarted` SpawnerManager (`|CreateDelegate` :!event `SpawnEnnemies`)))

(event `self.ReceiveBeginPlay`
  (bind _returnvalue (`GameplayStatics.GetActorOfClass` "/Game/Game/Ennemies/Spawner/BP_SpawnerManager.BP_SpawnerManager_C"))
  (`/Engine/EditorBlueprintResources/StandardMacros.IsValid` _returnvalue
    (:`Is Valid`
      (`self.OnSpawnerManagerCreated` _returnvalue))
    (:`Is Not Valid`
      (bind _returnvalue_2 (`GameplayStatics.GetActorOfClass` "/Game/Game/MainLevel/BP_GameManager.BP_GameManager_C"))
      (add `/Game/Game/MainLevel/BP_GameManager.SpawnerManagerCreated` _returnvalue_2 (`|CreateDelegate` :!event `OnSpawnerManagerCreated`)))))

(event `PopulateSpawner`
  (params (Ennemies :type Integer))
  (if (== Ennemies 0)
    (`KismetSystemLibrary.PrintString` "Your forgot to pass ennemies to populate me!")
    (else
      (set `self.NumberOfEnnemiesToSpawn` Ennemies))))

(event `SpawnEnnemies`
  (params (Zone :type Integer))
  (if (<= (`self.Zone`) Zone)
    (`self.SpawnSequence`)))

(event `SpawnSequence`
  (bind _returnvalue (`self.GetTransform`))
  (bind _spawnloopint (`self.SpawnLoopInt`))
  (bind _returnvalue_2 (`|SpawnActorFromClass` "/Game/Game/Ennemies/Blueprints/BP_Ennemy.BP_Ennemy_C" (`KismetMathLibrary.MakeTransform` (`KismetMathLibrary.MakeVector` (.x (.location _returnvalue)) (.y (.location _returnvalue)) (+ (.z (.location _returnvalue)) (* (.z (.location _returnvalue)) (`self.SpawnLoopInt`)))) (.rotation _returnvalue) (.scale _returnvalue)) "Undefined" "MultiplyWithRoot" null null))
  (`/Engine/EditorBlueprintResources/StandardMacros.IsValid` _returnvalue_2
    (:`Is Valid`
      (`Pawn.SpawnDefaultController` _returnvalue_2)
      (`KismetSystemLibrary.Delay` (* (`KismetMathLibrary.RandomFloat`) (`self.MaxWaitingSpawnTime`)))
      (`/Engine/EditorBlueprintResources/StandardMacros.IncrementInt` _spawnloopint
        (:`  `
          (if (< _spawnloopint (`self.NumberOfEnnemiesToSpawn`))
            (`self.SpawnSequence`)))))))

(fn `UserConstructionScript`)