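; Spawner manager that drives enemy waves from the game's buy-time and combat state changes.
; On BeginPlay it finds BP_GameManager and binds to its state change, destroying all BP_Ennemy actors when buy time starts.
; When buy time ends, it broadcasts OnWaveStarted with the manager's unlocked zone.
; OnSpawnerAdded populates the given spawner with a fixed count; its switch on zone has empty branches.
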(event `self.ReceiveBeginPlay`
  (`self.EnableInput` (`GameplayStatics.GetPlayerController` 0))
  (bind _returnvalue (`GameplayStatics.GetActorOfClass` "/Game/Game/MainLevel/BP_GameManager.BP_GameManager_C"))
  (bind _output_get (set `self.GameManager` _returnvalue))
  (add `/Game/Game/MainLevel/BP_GameManager.OnGameStateChanged` _output_get (delegate `OnStateChanged`)))

(event `OnStateChanged`
  (params (IsBuyingTime :type Boolean))
  (if IsBuyingTime
    (bind _outactors (`GameplayStatics.GetAllActorsOfClass` "/Game/Game/Ennemies/Blueprints/BP_Ennemy.BP_Ennemy_C"))
    (for _array_element _outactors
      (`/Engine/EditorBlueprintResources/StandardMacros.IsValid` _array_element
        (:`Is Valid`
          (`self.K2_DestroyActor` _array_element))))
    (else
      (`self.StartWave`))))

(event `StartWave`
  (`self.OnWaveStarted` (`/Game/Game/MainLevel/BP_GameManager.UnlockedZone` (`self.GameManager`))))

(event `OnSpawnerAdded`
  (params (Spawner :type "/Game/Game/Ennemies/Spawner/BP_EnnemySpawner Object Reference"))
  (switch `int` (`/Game/Game/Ennemies/Spawner/BP_EnnemySpawner.Zone` Spawner)
    (:`Default`
      _)
    (:`0`
      _))
  (`/Game/Game/Ennemies/Spawner/BP_EnnemySpawner.PopulateSpawner` Spawner 10)
  (`KismetSystemLibrary.PrintString` "Spawner populated"))

(event `Key|SpaceBar`
  (params (Key :type "Key Structure")))

(fn `UserConstructionScript`)