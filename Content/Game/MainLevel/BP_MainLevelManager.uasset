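; Main level manager that alternates the game between a buying phase and a wave phase.
; Tick counts down the active phase's timer, and near zero resets it, flips IsBuyingTime and broadcasts OnGameStateChanged with the new flag.
; BeginPlay finds and caches the BP_SpawnerManager actor, which this graph does not use further.
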(event `self.ReceiveBeginPlay`
  (bind _returnvalue (`GameplayStatics.GetActorOfClass` "/Game/Game/Ennemies/Spawner/BP_SpawnerManager.BP_SpawnerManager_C"))
  (set `self.SpawnerManager` _returnvalue))

(event `self.ReceiveTick`
  (params (DeltaSeconds :type "Float (single-precision)"))
  (if (`self.IsBuyingTime`)
    (bind _output_get (set `self.BuyingTimer` (- (`self.BuyingTimer`) DeltaSeconds)))
    (if (<= _output_get 0.1)
      (set `self.BuyingTimer` (`self.InitialBuyingTimer`))
      (bind _output_get_2 (set `self.IsBuyingTime` false))
      (`self.OnGameStateChanged` _output_get_2))
    (else
      (bind _output_get_3 (set `self.WaveTimer` (- (`self.WaveTimer`) DeltaSeconds)))
      (if (<= _output_get_3 0.1)
        (set `self.WaveTimer` (`self.InitialWaveTimer`))
        (bind _output_get_4 (set `self.IsBuyingTime` true))
        (`self.OnGameStateChanged` _output_get_4)))))

(fn `UserConstructionScript`)