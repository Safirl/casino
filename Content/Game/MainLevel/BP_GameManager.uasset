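; BP_GameManager runs the main level's game loop, alternating timed buying phases and waves, and tracks zone unlocking.
; On BeginPlay it spawns and announces a BP_SpawnerManager.
; Tick counts down the active phase timer unless stopped, then resets it, flips the phase and broadcasts the change.
; Backspace increments the unlocked zone count, broadcasting each opened zone until the count exceeds three, when it signals the outside door to open.
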(event `self.ReceiveBeginPlay`
  (`self.EnableInput` (`GameplayStatics.GetPlayerController` 0))
  (bind _returnvalue (`|SpawnActorFromClass` "/Game/Game/Ennemies/Spawner/BP_SpawnerManager.BP_SpawnerManager_C" (`self.Spawn Transform`) "Undefined" "MultiplyWithRoot" null null))
  (bind _output_get (set `self.SpawnerManager` _returnvalue))
  (`self.SpawnerManagerCreated` _output_get))

(event `self.ReceiveTick`
  (params (DeltaSeconds :type "Float (single-precision)"))
  (if (`self.StopTimer`)
    _
    (elif (`self.IsBuyingTime`)
      (bind _output_get (set `self.BuyingTimer` (- (`self.BuyingTimer`) DeltaSeconds)))
      (if (<= _output_get 0.1)
        (set `self.BuyingTimer` (`self.InitialBuyingTimer`))
        (bind _output_get_2 (set `self.IsBuyingTime` false))
        (`self.OnGameStateChanged` _output_get_2)
        (`KismetSystemLibrary.PrintString` "start wave"))
      (else
        (bind _output_get_3 (set `self.WaveTimer` (- (`self.WaveTimer`) DeltaSeconds)))
        (if (<= _output_get_3 0.1)
          (set `self.WaveTimer` (`self.InitialWaveTimer`))
          (bind _output_get_4 (set `self.IsBuyingTime` true))
          (`self.OnGameStateChanged` _output_get_4)
          (`KismetSystemLibrary.PrintString` "start buy"))))))

(event `Key|BackSpace`
  (params (Key :type "Key Structure"))
  (:`Pressed`
    (`self.UnlockZone`)))

(event `UnlockZone`
  (bind _result (`/Engine/EditorBlueprintResources/StandardMacros.IncrementInt` (`self.UnlockedZone`))
    (:`  `
      (if (> _result 3)
        (`self.OpenOutiseDoor`)
        (else
          (`self.OnZoneOpened` (`self.UnlockedZone`)))))))

(event `OpenOutiseDoor`
  (`self.OnOutSideDoorIsOpen`))

(fn `UserConstructionScript`)