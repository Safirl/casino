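; BP_Key is a pickup key that unlocks a zone through BP_GameManager when BP_FirstPersonCharacter overlaps it, then plays a sound and destroys itself.
; On BeginPlay it registers itself with the character through AddActorToRender.
; A self-restarting timeline spins the cube and lerps the actor toward a point above the location captured at the start of each cycle.
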(event `self.ReceiveBeginPlay`
  (`self.KeyAnim`)
  (bind _returnvalue (`GameplayStatics.GetActorOfClass` "/Game/FirstPerson/Blueprints/BP_FirstPersonCharacter.BP_FirstPersonCharacter_C"))
  (`/Game/FirstPerson/Blueprints/BP_FirstPersonCharacter.AddActorToRender` _returnvalue self))

(event `self.ReceiveActorBeginOverlap`
  (params (OtherActor :type "Actor Object Reference"))
  (cast `/Game/FirstPerson/Blueprints/BP_FirstPersonCharacter` OtherActor)
  (bind _returnvalue (`GameplayStatics.GetActorOfClass` "/Game/Game/MainLevel/BP_GameManager.BP_GameManager_C"))
  (`/Game/Game/MainLevel/BP_GameManager.UnlockZone` _returnvalue)
  (`GameplayStatics.PlaySound2D` "/Game/Game/Assets/Sounds/keySound.keySound" 1.0 1.0 0.0 null null)
  (`self.K2_DestroyActor`))

(event `KeyAnim`
  (bind _returnvalue_location (`KismetMathLibrary.BreakTransform` (`self.GetTransform`)))
  (bind _output_get (set `self.StartTransform` _returnvalue_location))
  (set `self.TargetTransform` (+ _output_get (0.0 0.0 30.0)))
  (bind (_direction _newtrack_0) (`Timeline|Anim` :`NewTime` (`GameplayStatics.GetWorldDeltaSeconds`) :!via `PlayFromStart`)
    (:`Update`
      (`SceneComponent.K2_AddLocalRotation` (`self.cube`) (struct :`Yaw` 1.0) false false)
      (`self.K2_SetActorLocation` (`KismetMathLibrary.VLerp` (`self.StartTransform`) (`self.TargetTransform`) _newtrack_0)))
    (:`Finished`
      (`self.KeyAnim`))))

(fn `UserConstructionScript`)