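; BP_Cocktail is a health pickup that spins in place and restores life to the first-person character that touches it.
; On BeginPlay it finds BP_FirstPersonCharacter and registers itself through AddActorToRender.
; Tick adds yaw at a steady, frame-rate-independent speed.
; Its SphereCollision overlap casts to the character, calls AddLife with a fixed amount, then destroys the pickup.
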(event `self.ReceiveBeginPlay`
  (bind _returnvalue (`GameplayStatics.GetActorOfClass` "/Game/FirstPerson/Blueprints/BP_FirstPersonCharacter.BP_FirstPersonCharacter_C"))
  (`/Game/FirstPerson/Blueprints/BP_FirstPersonCharacter.AddActorToRender` _returnvalue self))

(event `self.ReceiveActorBeginOverlap`
  (params (OtherActor :type "Actor Object Reference")))

(event `self.ReceiveTick`
  (params (DeltaSeconds :type "Float (single-precision)"))
  (bind (_returnvalue_roll _returnvalue_pitch _returnvalue_yaw) (`KismetMathLibrary.BreakRotator` (`self.K2_GetActorRotation`)))
  (`self.K2_SetActorRotation` (`KismetMathLibrary.MakeRotator` _returnvalue_roll _returnvalue_pitch (+ _returnvalue_yaw (* DeltaSeconds 100.0)))))

(event `self.SphereCollision.OnComponentBeginOverlap`
  (params (OverlappedComponent :type "PrimitiveComponent Object Reference") (OtherActor :type "Actor Object Reference") (OtherComp :type "PrimitiveComponent Object Reference") (OtherBodyIndex :type Integer) (bFromSweep :type Boolean) (SweepResult :type "HitResult Structure (by ref)"))
  (bind _asbp_first_person_character (cast `/Game/FirstPerson/Blueprints/BP_FirstPersonCharacter` OtherActor))
  (`/Game/FirstPerson/Blueprints/BP_FirstPersonCharacter.AddLife` _asbp_first_person_character 10.0)
  (`self.K2_DestroyActor`))

(fn `UserConstructionScript`)